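; BP_BasePlayerInteractable is, by its name, a base Blueprint for player interactables, holding an activated or deactivated state.
; Activate, Deactivate and SetActivated are guarded setters that aim to call UpdateAfterChange only when the state changes.
; UpdateAfterChange shows the state by swapping a configurable material slot on the StaticMesh between activated and deactivated materials.
; A debug print of the state exists but is disconnected.
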(fn `Activate`
  (if (not (`self.isActivated`))
    (set `self.isActivated` true)
    (`self.UpdateAfterChange`)))

(fn `Deactivate`
  (if (`self.isActivated`)
    (set `self.isActivated` false)
    (`self.UpdateAfterChange`)))

(fn `SetActivated`
  (params (isActivated :type Boolean))
  (if (not (== isActivated (`self.isActivated`)))
    (set `self.isActivated` isActivated)
    (`self.UpdateAfterChange`)))

(fn `UpdateAfterChange`
  (`PrimitiveComponent.SetMaterial` (`self.StaticMesh`) (`self.MaterialIndexToChange`) (select `bool` (`self.isActivated`) :`false` (`self.DeactivatedMaterial`) :`true` (`self.ActivatedMaterial`) :!type "MaterialInterface Object Reference")))

(fn `UserConstructionScript`)